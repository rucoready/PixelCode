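; BP_Portal_Dungeon1 is a dungeon portal actor in the boss map gate set that switches on when its trigger box is overlapped.
; Any overlap on BoxOnCollision calls afterDestroy, which runs OverlapCollision on the BP_PortalCollision1 actors in the level and activates the NSGpuPortal effect.
; An older destroy-and-delay chain remains in the graph but is disconnected.
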(event `self.ReceiveBeginPlay`)

(event `afterDestroy`
  (bind _outactors (`GameplayStatics.GetAllActorsOfClass` "/Game/KMS_AI/BossMap/Gate/BP_PortalCollision1.BP_PortalCollision1_C"))
  (`/Game/KMS_AI/BossMap/Gate/BP_PortalCollision1.OverlapCollision` _outactors)
  (`ActorComponent.SetActive` (`self.NS_GpuPortal`) (`self.True`) false))

(event `self.BoxOnCollision.OnComponentBeginOverlap`
  (params (OverlappedComponent :type "PrimitiveComponent Object Reference") (OtherActor :type "Actor Object Reference") (OtherComp :type "PrimitiveComponent Object Reference") (OtherBodyIndex :type Integer) (bFromSweep :type Boolean) (SweepResult :type "HitResult Structure (by ref)"))
  (`self.afterDestroy`))

(fn `UserConstructionScript`)