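; BP_BouncySphere is an actor in the FluidNinja Niagara use cases that moves its static mesh back and forth in a continuous bounce.
; BeginPlay caches the mesh's relative location, and Tick accumulates time to offset it by a cosine wave driven by Frequency and Amplitude.
; RotBounceDirection switches the motion from local Z to local Y, and the move is applied without sweep.
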(event `self.ReceiveBeginPlay`
  (set `self.LocalPos` (`SceneComponent.RelativeLocation` (`self.StaticMeshComponent`))))

(event `self.ReceiveTick`
  (params (DeltaSeconds :type "Float (single-precision)"))
  (bind _output_get (set `self.Time` (+ DeltaSeconds (`self.Time`))))
  (bind _returnvalue (* (* (`KismetMathLibrary.Cos` (* _output_get (`self.Frequency`))) (* (`self.Amplitude`) -1.0)) 100.0))
  (`SceneComponent.K2_SetRelativeLocation` (`self.StaticMeshComponent`) (+ (`KismetMathLibrary.SelectVector` (`KismetMathLibrary.MakeVector` 0.0 _returnvalue) (`KismetMathLibrary.MakeVector` 0.0 0.0 _returnvalue) (`self.RotBounceDirection`)) (`self.LocalPos`)) false false))

(fn `UserConstructionScript`)