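; FluidNinja utility actor that configures viewing and input for a level at runtime.
; BeginPlay, unless disabled, applies camera speed and quality/FPS console overrides, optionally possesses the nearest other Pawn, adds a directional-light rotator widget and can suppress UE5.1 TSR smearing.
; Keys step global time dilation, cutting motion blur at zero, while mouse buttons switch input modes, cursor visibility and look input.
; Construction script colors the editor icon by disabled state.
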(event `Key|Add` :consume false
  (params (Key :type "Key Structure"))
  (bind _customtimedilation (`self.CustomTimeDilation`))
  ;[0.04688 0.04688 0.04688] Time Dilation (slow down/pause Gameplay)
  (:`Pressed`
    (set `self.CustomTimeDilation` (+ _customtimedilation 0.25))
    (`GameplayStatics.SetGlobalTimeDilation` _customtimedilation :!label _label)
    (`KismetSystemLibrary.PrintString` (`KismetStringLibrary.Concat_StrStr` "Time dilation: " (`KismetStringLibrary.Conv_DoubleToString` (stale `Key|Subtract` _output_get))) (`self.Show Time Dilation Messages on Screen`) false (struct :`G` 0.66 :`B` 1.0 :`A` 1.0) 0.5)
    ;;[0.03646 0.03646 0.03646 1 12] Kills MotionBlur IF scene is stopped (TimeDilation = 0)
    (`KismetSystemLibrary.ExecuteConsoleCommand` (`KismetStringLibrary.Concat_StrStr` "r.DefaultFeature.MotionBlur " (`KismetStringLibrary.Conv_IntToString` (* (`self.MotionBlurQuality`) (`KismetMathLibrary.Conv_BoolToInt` (!= (stale `Key|Subtract` _output_get) 0.0))))) null)))

(event `Key|Subtract` :consume false
  (params (Key :type "Key Structure"))
  ;[0.04688 0.04688 0.04688] Time Dilation (slow down/pause Gameplay)
  (:`Pressed`
    (bind _output_get (set `self.CustomTimeDilation` (- (`self.CustomTimeDilation`) 0.25)))
    (goto _label)))

(event `Key|LeftMouseButton` :consume false
  (params (Key :type "Key Structure"))
  (bind _returnvalue (`GameplayStatics.GetPlayerController` 0))
  ;[0.1406 0.1406 0.1406] Cursor Visibility VS Camera Lagging
  (:`Pressed`
    (`WidgetBlueprintLibrary.SetInputMode_GameOnly` _returnvalue)
    (`Controller.SetIgnoreLookInput` _returnvalue true)
    (`WidgetBlueprintLibrary.SetInputMode_GameAndUIEx` _returnvalue null "DoNotLock" false :!label _label_2))
  (:`Released`
    (`Controller.SetIgnoreLookInput` _returnvalue false)))

(event `Key|MiddleMouseButton` :consume false
  (params (Key :type "Key Structure"))
  (bind _returnvalue (`GameplayStatics.GetPlayerController` 0))
  ;[0.1406 0.1406 0.1406] Cursor Visibility VS Camera Lagging
  (:`Pressed`
    (`WidgetBlueprintLibrary.SetInputMode_GameOnly` _returnvalue :!label _label_3)
    (set `PlayerController.bShowMouseCursor` false _returnvalue))
  (:`Released`
    (set `PlayerController.bShowMouseCursor` (`self.ShowMouseCursor`) _returnvalue :!label _label_4)
    (goto _label_2)))

(event `Key|RightMouseButton` :consume false
  (params (Key :type "Key Structure"))
  ;[0.1406 0.1406 0.1406] Cursor Visibility VS Camera Lagging
  (:`Pressed`
    (goto _label_3))
  (:`Released`
    (goto _label_4)))

(event `self.ReceiveBeginPlay`
  (bind _returnvalue (`GameplayStatics.GetPlayerPawn` 0))
  (bind _returnvalue_2 (`GameplayStatics.GetPlayerController` 0))
  (bind _returnvalue_3 (`GameplayStatics.GetPlayerController` 0))
  (bind _widgettorotatedirectionallight (`self.WidgetToRotateDirectionalLight`))
  (bind _temparray1 (`self.TempArray1`))
  (bind _rootcomponent (`Actor.RootComponent` (`Controller.K2_GetPawn` _returnvalue_3)))
  (if (not (`self.DisableBlueprint`))
    (`|ExecutionSequence`
      (:`then_0`
        ;[0.1406 0.1406 0.1406] Cursor Visibility VS Camera Lagging
        (if (`self.CameraAndCursorSmoothing`)
          (`self.EnableInput` _returnvalue_2)
          (set `PlayerController.bShowMouseCursor` (`self.ShowMouseCursor`) _returnvalue_2)
          (goto _label_2)))
      (:`then_1`
        ;[0.1927 0.1927 0.1927 1 14] Set Camera movement speed
        (bind _asfloating_pawn_movement (cast `FloatingPawnMovement` (`Pawn.GetMovementComponent` (`GameplayStatics.GetPlayerPawn` 0))))
        (set `FloatingPawnMovement.MaxSpeed` (`KismetMathLibrary.Conv_IntToDouble` (`self.MaxCameraMoveSpeed`)) _asfloating_pawn_movement))
      (:`then_2`
        (`|ExecutionSequence`
          (:`then_0`
            ;[1 0 0.1187 1 14] Execute console commands
            (if (`self.OverrideEditor120-FPS-Limit`)
              (`KismetSystemLibrary.ExecuteConsoleCommand` (`KismetStringLibrary.Concat_StrStr` "t.MaxFPS " (`KismetStringLibrary.Conv_IntToString` (`self.MaxEditorFPS`))) null)))
          (:`then_1`
            (`KismetSystemLibrary.ExecuteConsoleCommand` (`KismetStringLibrary.Concat_StrStr` "sg.AntiAliasingQuality" (`KismetStringLibrary.Conv_IntToString` (`self.AntialiasingQuality`))) null)
            (`KismetSystemLibrary.ExecuteConsoleCommand` (`KismetStringLibrary.Concat_StrStr` "r.DepthOfFieldQuality " (`KismetStringLibrary.Conv_IntToString` (`self.DepthOfFieldQuality`))) null)
            (`KismetSystemLibrary.ExecuteConsoleCommand` (`KismetStringLibrary.Concat_StrStr` "r.DefaultFeature.MotionBlur " (`KismetStringLibrary.Conv_IntToString` (`self.MotionBlurQuality`))) null))))
      (:`then_3`
        ;[0.1771 0.1771 0.1771] Possess nearest Pawn
        (if (`self.PossessNearestPawn`)
          (bind _outactors (`GameplayStatics.GetAllActorsOfClass` "/Script/Engine.Pawn"))
          (if (!= (`KismetArrayLibrary.Array_Length` _outactors) 0)
            (for _array_element _outactors
              (if (not (== _array_element _returnvalue))
                (`KismetArrayLibrary.Array_Add` (`self.TempArray2`) _array_element)
                (`KismetArrayLibrary.Array_Add` _temparray1 (`KismetMathLibrary.Abs_Int` (`KismetMathLibrary.FTrunc` (`self.GetDistanceTo` _array_element _returnvalue))))))
            (`|ExecutionSequence`
              (:`then_0`
                ;;[1 0 0 1 14] Remove the Default Pawn's collision object - so it won't interfere with the new camera
                ;; (Def.Pawn is a camera with a sphere - and this sphere is visible once you leave the POV)
                (`SceneComponent.K2_SetWorldLocation` _rootcomponent (0.0 0.0 0.0) false false)
                (`SceneComponent.SetVisibility` _rootcomponent false true))
              (:`then_1`
                (`Controller.Possess` _returnvalue_3 (`|GetArrayItem` (`self.TempArray2`) (`KismetMathLibrary.MinOfIntArray` _temparray1))))))))
      (:`then_4`
        ;[0.1771 0.1771 0.1771] Add Light Rotator Widget to Screen (Lower right corner)
        (if (`KismetSystemLibrary.IsValidClass` _widgettorotatedirectionallight)
          (bind _returnvalue_4 (`|CreateWidget` _widgettorotatedirectionallight (`GameplayStatics.GetPlayerController` 0)))
          (bind _asbp_viewport_light_rotator_widget (cast `/Game/FluidNinja/Core/BP_Viewport_LightRotatorWidget` _returnvalue_4))
          (set `/Game/FluidNinja/Core/BP_Viewport_LightRotatorWidget.DirectionalLight` (`self.WidgetTargetDirectionalLight`) _asbp_viewport_light_rotator_widget)
          (`UserWidget.AddToViewport` _returnvalue_4 1)))
      (:`then_5`
        ;[1 0.0296 0] SupressUE51TextureSmearing
        (if (`self.SupressUE51TextureSmearing`)
          (`KismetSystemLibrary.ExecuteConsoleCommand` "r.TSR.ShadingRejection.Flickering 0" null)
          (`KismetSystemLibrary.ExecuteConsoleCommand` "r.TSR.ShadingRejection.Flickering.Period 0" null))))))

(event `Key|Escape`
  (params (Key :type "Key Structure"))
  ;[0 0 0] On Quit Enable DOF and Mblur
)

(fn `UserConstructionScript`
  (bind _editoricon (`self.EditorIcon`))
  ;[0.1354 0.1354 0.1354] Set Editor Icon Color
  (if (`self.DisableBlueprint`)
    (`PrimitiveComponent.SetMaterial` _editoricon 0 "/Game/FluidNinja/Core/GUI/MI_FluidNinjaLogo_Gray.MI_FluidNinjaLogo_Gray")
    (else
      (`PrimitiveComponent.SetMaterial` _editoricon 0 "/Game/FluidNinja/Core/GUI/MI_FluidNinjaLogo_Green.MI_FluidNinjaLogo_Green"))))