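; An example child building actor for the building system, representing a snappable cube.
; It overrides BuildingInfos to hand the parent its collision box, two hit-control arrows and two snap scene components.
; Tick and construction only defer to the parent, so placement and snapping logic is not defined here.
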(event `self.ReceiveTick`
  (params (DeltaSeconds :type "Float (single-precision)"))
  (`parent.ReceiveTick` DeltaSeconds))

(fn `BuildingInfos`
  (returns (CheckBoxCollisions :type "Array of BoxComponent Object Reference") (CheckSphereCollisions :type "Array of SphereComponent Object Reference") (CheckArrowComponent :type "Array of ArrowComponent Object Reference") (SnapSceneComponents :type "Array of SceneComponent Object Reference"))
  (return (`|MakeArray` (`self.Box`)) _ (`|MakeArray` (`self.HitControlArrow`) (`self.HitControlArrow2`)) (`|MakeArray` (`self.SnapScene1`) (`self.SnapScene2`))))

(fn `UserConstructionScript`
  (`parent.UserConstructionScript`))