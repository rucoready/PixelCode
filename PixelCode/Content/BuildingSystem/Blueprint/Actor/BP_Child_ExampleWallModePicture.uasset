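; Example child building piece, apparently a wall-mounted picture for the building system's wall mode.
; It overrides BuildingInfos to supply its Box component as the collision check and HitControlArrow as the arrow check component.
; The construction script only calls the parent, and the event graph holds only disabled stub events.
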(fn `BuildingInfos`
  (returns (CheckBoxCollisions :type "Array of BoxComponent Object Reference") (CheckSphereCollisions :type "Array of SphereComponent Object Reference") (CheckArrowComponent :type "Array of ArrowComponent Object Reference") (SnapSceneComponents :type "Array of SceneComponent Object Reference"))
  (return (`|MakeArray` (`self.Box`)) _ (`|MakeArray` (`self.HitControlArrow`))))

(fn `UserConstructionScript`
  (`parent.UserConstructionScript`))