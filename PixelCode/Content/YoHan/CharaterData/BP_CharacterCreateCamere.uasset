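; Camera pawn for the character creation screen, which adds the CharaterCreateUI widget to the viewport on BeginPlay.
; Mouse X and Y drive controller yaw and pitch, with the control rotation's roll reset to zero on the X axis event.
; Mouse wheel down lengthens the spring arm within clamped limits to zoom out; no wheel-up handler is present.
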(event `self.ReceiveBeginPlay`
  (bind _returnvalue (`|CreateWidget` "/Game/YoHan/CharaterData/CharaterCreateUI.CharaterCreateUI_C"))
  (`UserWidget.AddToViewport` _returnvalue 0))

(event `InputAxisKey|MouseX`
  (params (AxisValue :type "Float (single-precision)"))
  (bind (_returnvalue_roll _returnvalue_pitch _returnvalue_yaw) (`KismetMathLibrary.BreakRotator` (`self.GetControlRotation`)))
  ;[1 1 1] Moverment for camera
  (`self.AddControllerYawInput` AxisValue)
  (`Controller.SetControlRotation` (`GameplayStatics.GetPlayerController` 0) (`KismetMathLibrary.MakeRotator` 0.0 _returnvalue_pitch _returnvalue_yaw)))

(event `InputAxisKey|MouseY`
  (params (AxisValue :type "Float (single-precision)"))
  ;[1 1 1] Moverment for camera
  (`self.AddControllerPitchInput` AxisValue))

(event `Key|MouseScrollDown`
  (params (Key :type "Key Structure"))
  (bind _springarm (`self.SpringArm`))
  (:`Pressed`
    (set `SpringArmComponent.TargetArmLength` (`KismetMathLibrary.FClamp` (- (`SpringArmComponent.TargetArmLength` _springarm) -20.0) (`self.Min`) (`self.Max`)) _springarm)))

(event `Key|MouseScrollUp`
  (params (Key :type "Key Structure")))

(fn `UserConstructionScript`)