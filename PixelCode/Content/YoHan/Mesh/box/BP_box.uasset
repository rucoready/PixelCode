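; BP_box is a box actor that swings open when the player character hits it.
; A hit on the Box1 component checks for player character 0, then calls the OpenBox event.
; OpenBox plays a timeline that drives the Box component's relative rotation, lerping from the actor's current rotation to a fixed target angle.
; No closing logic is present.
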(event `OpenBox`
  (bind (_direction _newtrack_0) (`Timeline|Timeline`)
    (:`Update`
      (`SceneComponent.K2_SetRelativeRotation` (`self.Box`) (`KismetMathLibrary.RLerp` (`self.K2_GetActorRotation`) (struct :`Roll` -120.0) _newtrack_0) false false))))

(event `self.Box1.OnComponentHit`
  (params (HitComponent :type "PrimitiveComponent Object Reference") (OtherActor :type "Actor Object Reference") (OtherComp :type "PrimitiveComponent Object Reference") (NormalImpulse :type "Vector Structure") (Hit :type "HitResult Structure (by ref)"))
  (if (== OtherActor (`GameplayStatics.GetPlayerCharacter` 0))
    (`self.OpenBox`)))

(fn `UserConstructionScript`)