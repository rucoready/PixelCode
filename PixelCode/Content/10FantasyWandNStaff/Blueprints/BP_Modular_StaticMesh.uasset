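; Modular static mesh actor that assembles a prop, likely a fantasy wand or staff, from body, head and tail pieces.
; The construction script always adds the selected body mesh, then adds head and tail meshes only when their index is above zero.
; Each piece is a new static mesh component picked by index from a mesh array.
; Head and tail offsets are looked up by body index, with a uniform scale per piece.
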(event `Set Body Mesh`
  ;[1 1 1] Set Body Mesh
  (bind _returnvalue (`AddComponent|NODE_AddStaticMeshComponent-2`))
  (`StaticMeshComponent.SetStaticMesh` _returnvalue (`|GetArrayItem` (`self.mainBodyMesh`) (`self.mainBodyValue`))))

(event `Set Head Mesh`
  (bind _headscale (`self.headScale`))
  ;[1 1 1] Set Head Mesh
  (bind _returnvalue (`AddComponent|NODE_AddStaticMeshComponent-0` :`RelativeTransform` (`KismetMathLibrary.MakeTransform` (`|GetArrayItem` (`self.headLocation`) (`self.mainBodyValue`)) (struct) (`KismetMathLibrary.MakeVector` _headscale _headscale _headscale))))
  (`StaticMeshComponent.SetStaticMesh` _returnvalue (`|GetArrayItem` (`self.headMesh`) (`self.headValue`))))

(event `Set Tail Mesh`
  (bind _tailscale (`self.tailScale`))
  ;[1 1 1] Set Tail Mesh
  (bind _returnvalue (`AddComponent|NODE_AddStaticMeshComponent-1` :`RelativeTransform` (`KismetMathLibrary.MakeTransform` (`|GetArrayItem` (`self.tailLocation`) (`self.mainBodyValue`)) (struct) (`KismetMathLibrary.MakeVector` _tailscale _tailscale _tailscale))))
  (`StaticMeshComponent.SetStaticMesh` _returnvalue (`|GetArrayItem` (`self.tailMesh`) (`self.tailValue`))))

(fn `UserConstructionScript`
  (`self.Set Body Mesh`)
  (if (> (`self.HeadValue`) 0)
    (`self.Set Head Mesh`))
  (if (> (`self.TailValue`) 0)
    (`self.Set Tail Mesh`)))