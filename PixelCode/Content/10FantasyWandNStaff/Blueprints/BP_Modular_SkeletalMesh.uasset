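; Modular actor that assembles a skeletal mesh from interchangeable body, head and tail parts, chosen by index from mesh arrays.
; The construction script always adds the body, then adds head and tail components when their values exceed zero, with per-body offsets and adjustable uniform scale.
; Heads flagged as animated loop their assigned animation at BeginPlay and whenever the head mesh is set.
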(event `self.ReceiveBeginPlay`
  ;[1 1 1] Check for Head Animation.
  (if (`|GetArrayItem` (`self.AnimatedHeadMesh?`) (`self.HeadValue`)) :!label _label
    (`SkeletalMeshComponent.PlayAnimation` (`self.Ref-HeadMesh`) (`|GetArrayItem` (`self.AnimationToPlay`) (`self.HeadValue`)) true)))

(event `CheckHeadAnim`
  ;[1 1 1] Check for Head Animation.
  (goto _label))

(event `Set Body Mesh`
  ;[1 1 1] Set Body Mesh
  (bind _returnvalue (`AddComponent|NODE_AddSkeletalMeshComponent-1`))
  (`SkinnedMeshComponent.SetSkinnedAssetAndUpdate` _returnvalue (`|GetArrayItem` (`self.MainBodyMesh`) (`self.MainBody-Value`)) true))

(event `Set Head Mesh`
  (bind _headscale (`self.HeadScale`))
  ;[1 1 1] Set Head Mesh
  (bind _returnvalue (`AddComponent|NODE_AddSkeletalMeshComponent-2` :`RelativeTransform` (`KismetMathLibrary.MakeTransform` (`|GetArrayItem` (`self.HeadLocation`) (`self.MainBody-Value`)) (struct) (`KismetMathLibrary.MakeVector` _headscale _headscale _headscale))))
  (bind _output_get (set `self.Ref-HeadMesh` _returnvalue))
  (`SkinnedMeshComponent.SetSkinnedAssetAndUpdate` _output_get (`|GetArrayItem` (`self.HeadMesh`) (`self.HeadValue`)) true)
  ;[1 1 1] This is just to play animation if you change head value during play.
  (`self.CheckHeadAnim`))

(event `Set Tail Mesh`
  (bind _tailscale (`self.TailScale`))
  ;[1 1 1] Set Tail Mesh
  (bind _returnvalue (`AddComponent|NODE_AddSkeletalMeshComponent-0` :`RelativeTransform` (`KismetMathLibrary.MakeTransform` (`|GetArrayItem` (`self.TailLocation`) (`self.MainBody-Value`)) (struct) (`KismetMathLibrary.MakeVector` _tailscale _tailscale _tailscale))))
  (bind _output_get (set `self.Ref-TailMesh` _returnvalue))
  (`SkinnedMeshComponent.SetSkinnedAssetAndUpdate` _output_get (`|GetArrayItem` (`self.TailMesh`) (`self.TailValue`)) true))

(fn `UserConstructionScript`
  (`self.Set Body Mesh`)
  (if (> (`self.HeadValue`) 0)
    (`self.Set Head Mesh`))
  (if (> (`self.TailValue`) 0)
    (`self.Set Tail Mesh`)))