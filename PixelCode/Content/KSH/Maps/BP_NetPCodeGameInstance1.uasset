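; Game instance that keeps placed-building data in a save slot and can apply a stored skeletal mesh to the player character.
; On Init it loads the existing BP_Saver save or creates a new one.
; The add and remove building events edit that save's building collection and immediately write it back to the slot.
; SetCharacter casts player 0 to BP_Player and swaps its mesh.
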(event `Set Character`
  (bind (_newvar_icon _newvar_skeletalmesh) (break `ItemAssetDatas` (`self.NewVar`)))
  (bind _asbp_player (cast `/Game/Player/Blueprint/BP_Player` (`GameplayStatics.GetPlayerCharacter` 0)))
  (`SkeletalMeshComponent.SetSkeletalMeshAsset` (`Character.Mesh` _asbp_player) _newvar_skeletalmesh))

(event `self.ReceiveInit`
  ;[1 1 1] 빌딩 데이터가 있는지 확인 후 로드
  (bind _returnvalue (`GameplayStatics.DoesSaveGameExist` (`self.SavedBuildingDataName`)))
  (if _returnvalue
    (bind _returnvalue_2 (`GameplayStatics.LoadGameFromSlot` (`self.SavedBuildingDataName`)))
    (bind _asbp_saver (cast `/Game/KSH/Maps/BP_Saver` _returnvalue_2))
    (set `self.BP SaveRef` _asbp_saver)
    (else
      (bind _returnvalue_3 (`GameplayStatics.CreateSaveGameObject` "/Game/KSH/Maps/BP_Saver.BP_Saver_C"))
      (set `self.BP SaveRef` _returnvalue_3))))

(event `BP_AddBuildingData`
  (params (NewParam :type "/Game/KSH/Maps/ST_BuildingData Structure"))
  (`KismetArrayLibrary.Array_Add` (`/Game/KSH/Maps/BP_Saver.Buildings_BPVar` (`self.BP SaveRef`)) NewParam)
  (`GameplayStatics.SaveGameToSlot` (`self.BP SaveRef`) (`self.SavedBuildingDataName`)))

(event `BP_RemoveBuildingData`
  (params (NewParam :type "/Game/KSH/Maps/ST_BuildingData Structure"))
  (`KismetArrayLibrary.Array_RemoveItem` (`/Game/KSH/Maps/BP_Saver.Buildings_BPVar` (`self.BP SaveRef`)) NewParam)
  (`GameplayStatics.SaveGameToSlot` (`self.BP SaveRef`) (`self.SavedBuildingDataName`)))