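; BP_Building is a building actor with an instanced foundation mesh, used here as a testbed for placing objects at sockets on individual mesh instances.
; BeginPlay and the construction script are empty, so none of the graph logic runs.
; One disconnected experiment spawns BP_TestCube at an instance socket transform through GetInstancedSocketTransform after a delay.
; An older one manually combines instance and socket transforms to add a static mesh component.
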(event `self.ReceiveBeginPlay`)

(fn `UserConstructionScript`)