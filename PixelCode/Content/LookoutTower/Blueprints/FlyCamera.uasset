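; FlyCamera is a fly-camera pawn for the LookoutTower content, with its travel speed adjustable by mouse wheel.
; Wheel up and wheel down presses raise or lower the FloatingPawnMovement MaxSpeed by the Step variable, with no clamping in the graph.
; The graph contains no movement or look logic, and its BeginPlay, overlap, Tick and construction script are empty.
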(event `Key|MouseScrollUp`
  (params (Key :type "Key Structure"))
  (bind _floatingpawnmovement (`self.FloatingPawnMovement`))
  (:`Pressed`
    (set `FloatingPawnMovement.MaxSpeed` (+ (`MovementComponent.GetMaxSpeed` _floatingpawnmovement) (`self.Step`)) _floatingpawnmovement)))

(event `Key|MouseScrollDown`
  (params (Key :type "Key Structure"))
  (bind _floatingpawnmovement (`self.FloatingPawnMovement`))
  (:`Pressed`
    (set `FloatingPawnMovement.MaxSpeed` (- (`MovementComponent.GetMaxSpeed` _floatingpawnmovement) (`self.Step`)) _floatingpawnmovement)))

(fn `UserConstructionScript`)