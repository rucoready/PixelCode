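; Interactive furniture Blueprint for a chest with seven drawers that slide open and closed independently.
; FurnitureTrace prints a "Press E" prompt, and FurnitureAction compares the traced component against each drawer mesh.
; The matched drawer's FlipFlop plays or reverses its own timeline, which lerps the mesh's relative location along local Y between hardcoded closed and open positions.
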(event `/Game/LookoutTower/Blueprints/Character/BP_Demo_Interface.FurnitureTrace`
  ;[1 1 1] DebugInfo
  (`KismetSystemLibrary.PrintText` "Press E" true false (struct :`R` 1.0 :`G` 1.0 :`B` 1.0 :`A` 1.0) 0.0))

(event `/Game/LookoutTower/Blueprints/Character/BP_Demo_Interface.FurnitureAction`
  (params (TraceComponent :type "SceneComponent Object Reference"))
  (bind _staticmeshcomponent1 (`self.StaticMeshComponent1`))
  (bind _staticmeshcomponent5 (`self.StaticMeshComponent5`))
  (bind _staticmeshcomponent6 (`self.StaticMeshComponent6`))
  (bind _staticmeshcomponent7 (`self.StaticMeshComponent7`))
  (bind _staticmeshcomponent2 (`self.StaticMeshComponent2`))
  (bind _staticmeshcomponent3 (`self.StaticMeshComponent3`))
  (bind _staticmeshcomponent4 (`self.StaticMeshComponent4`))
  ;[1 1 1] InteractionPart
  (if (== TraceComponent _staticmeshcomponent1)
    (`/Engine/EditorBlueprintResources/StandardMacros.FlipFlop`
      (:`A`
        (bind (_direction _alpha) (`Timeline|Timeline_0` :!label _label)
          (:`Update`
            (`SceneComponent.K2_SetRelativeLocation` _staticmeshcomponent1 (`KismetMathLibrary.VLerp` (-40.426743 30.184338 17.748055) (-40.426743 60.184338 17.748055) _alpha) false false))))
      (:`B`
        (goto _label :!via `Reverse`)))
    (elif (== TraceComponent _staticmeshcomponent2)
      (`/Engine/EditorBlueprintResources/StandardMacros.FlipFlop`
        (:`A`
          (bind (_direction_2 _alpha_2) (`Timeline|Timeline_1` :!label _label_2)
            (:`Update`
              (`SceneComponent.K2_SetRelativeLocation` _staticmeshcomponent2 (`KismetMathLibrary.VLerp` (42.405941 30.046555 17.748055) (42.405941 60.046555 17.748055) _alpha_2) false false))))
        (:`B`
          (goto _label_2 :!via `Reverse`)))
      (elif (== TraceComponent _staticmeshcomponent3)
        (`/Engine/EditorBlueprintResources/StandardMacros.FlipFlop`
          (:`A`
            (bind (_direction_3 _alpha_3) (`Timeline|Timeline_2` :!label _label_3)
              (:`Update`
                (`SceneComponent.K2_SetRelativeLocation` _staticmeshcomponent3 (`KismetMathLibrary.VLerp` (55.927437 30.046547 55.263504) (55.927437 60.046547 55.263504) _alpha_3) false false))))
          (:`B`
            (goto _label_3 :!via `Reverse`)))
        (elif (== TraceComponent _staticmeshcomponent4)
          (`/Engine/EditorBlueprintResources/StandardMacros.FlipFlop`
            (:`A`
              (bind (_direction_4 _alpha_4) (`Timeline|Timeline_3` :!label _label_4)
                (:`Update`
                  (`SceneComponent.K2_SetRelativeLocation` _staticmeshcomponent4 (`KismetMathLibrary.VLerp` (0.612361 30.046532 55.204609) (0.612361 60.046532 55.204609) _alpha_4) false false))))
            (:`B`
              (goto _label_4 :!via `Reverse`)))
          (elif (== TraceComponent _staticmeshcomponent5)
            (`/Engine/EditorBlueprintResources/StandardMacros.FlipFlop`
              (:`A`
                (bind (_direction_5 _alpha_5) (`Timeline|Timeline_4` :!label _label_5)
                  (:`Update`
                    (`SceneComponent.K2_SetRelativeLocation` _staticmeshcomponent5 (`KismetMathLibrary.VLerp` (42.471004 30.18433 36.587543) (42.471004 60.18433 36.587543) _alpha_5) false false))))
              (:`B`
                (goto _label_5 :!via `Reverse`)))
            (elif (== TraceComponent _staticmeshcomponent6)
              (`/Engine/EditorBlueprintResources/StandardMacros.FlipFlop`
                (:`A`
                  (bind (_direction_6 _alpha_6) (`Timeline|Timeline_5` :!label _label_6)
                    (:`Update`
                      (`SceneComponent.K2_SetRelativeLocation` _staticmeshcomponent6 (`KismetMathLibrary.VLerp` (-40.471813 30.046539 36.598686) (-40.471813 60.046539 36.598686) _alpha_6) false false))))
                (:`B`
                  (goto _label_6 :!via `Reverse`)))
              (elif (== TraceComponent _staticmeshcomponent7)
                (`/Engine/EditorBlueprintResources/StandardMacros.FlipFlop`
                  (:`A`
                    (bind (_direction_7 _alpha_7) (`Timeline|Timeline_6` :!label _label_7)
                      (:`Update`
                        (`SceneComponent.K2_SetRelativeLocation` _staticmeshcomponent7 (`KismetMathLibrary.VLerp` (-54.565323 30.046555 55.263504) (-54.565323 60.046555 55.263504) _alpha_7) false false))))
                  (:`B`
                    (goto _label_7 :!via `Reverse`)))))))))))

(fn `UserConstructionScript`)